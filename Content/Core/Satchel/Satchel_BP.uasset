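; Satchel_BP is a throwable explosive charge that is launched and detonated through custom events.
; ThrowSatchel sets projectile velocity from the aim direction plus half the instigator's velocity.
; Detonate spawns a blast effect, plays the BOMB audio event, fires a radial force impulse and destroys the actor.
; A three-second auto-detonate chain is disconnected, and the SatchelIndicate function is an empty stub.
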(event Custom|Detonate
  ;[0.15 0.1319 0 0.5] Detonate Logic
  (Game|SpawnActorfromClass "/Game/Core/Satchel/BlastFX.BlastFX_C" (Math|Transform|MakeTransform (+ (Transformation|GetActorLocation) "0.000000,0.000000,70.000000") "0, 0, 0" "1.500000,1.500000,1.500000") "Undefined" "MultiplyWithRoot" 0 0)
  (Class|FMODBlueprintStatics|PlayEventatLocation "/Game/FMOD/Events/BOMB.BOMB" (Transformation|GetActorTransform))
  (Class|RadialForceComponent|FireImpulse (Variables|Default|GetRadialForce))
  (Actor|DestroyActor))

(event Custom|ThrowSatchel
  (params (Direction :type Vector))
  ;[0 0.15 0.06205 0.5] Lauch Logic
  (Variables|/Script/Engine.MovementComponent|SetVelocity (Variables|Default|GetProjectileMovement) (+ (* Direction (Variables|/Script/Engine.ProjectileMovementComponent|GetInitialSpeed (Variables|Default|GetProjectileMovement))) (* (Transformation|GetVelocity (Game|GetInstigator)) 0.5)))
  (CallFunction|SatchelIndicate false))

(fn ConstructionScript)

(fn SatchelIndicate
  (params (IsSatchelActive :type Boolean))
  (return))