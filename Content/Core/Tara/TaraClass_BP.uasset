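; Tara is the player character of a timed movement game, with wall running, wall jumps and throwable, detonatable satchels.
; Hits on Wallrun-tagged surfaces start a plane-constrained run, kept alive each tick by input checks and traces, with an Arc timeline and optional reversible grip timer.
; Satchel charges refill on landing or while grounded.
; Level-name checks switch between tutorial dialogue and a stopwatch whose time saves to a leaderboard.
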(event OnComponentHit(CapsuleComponent)
  (params (HitComponent :type Primitive%20Component%20Object%20Reference) (OtherActor :type Actor%20Object%20Reference) (OtherComp :type Primitive%20Component%20Object%20Reference) (NormalImpulse :type Vector :default "0, 0, 0") (Hit :type Hit%20Result%20Structure%20%28by%20ref%29))
  (bind _impactnormal (Collision|BreakHitResult Hit))
  (bind _returnvalue (Transformation|GetActorRightVector))
  (bind _mesh (Variables|Character|GetMesh))
  (bind _returnvalue_2 (Math|Vector|DotProduct _impactnormal _returnvalue))
  (bind _returnvalue_3 (Transformation|GetWorldLocation _mesh))
  (bind _returnvalue_4 (> _returnvalue_2 0.0))
  ;[0 0.008023 0.15 0.502] Wallrun
  ;;[0 0.008023 0.15 0.502] Start Wallrunning when detecting a hit
  (if (Actor|ActorHasTag OtherActor "Wallrun")
    (if (not (and (not (Variables|Default|GetbIsWallRunning)) (not (AI|Components|NavMovement|IsFalling (Variables|Character|GetCharacterMovement)))))
      (Variables|WallRunning|SetWallRunNormal (Math|Vector|CrossProduct _impactnormal (select _returnvalue_4 "0.000000,0.000000,1.000000" "0.000000,0.000000,-1.000000")))
      (Variables|WallRunning|SetWallRunDirection (select _returnvalue_4 "NewEnumerator1" "NewEnumerator0"))
      (if (and (CallFunction|ContinueWallrun?) (> (Math|Vector|DotProduct (Math|Vector|GetForwardVector (.Fixxed (CallFunction|GetInputDirection))) (Variables|WallRunning|GetWallRunNormal)) 0.4))
        (bind _returnvalue_5 (Collision|SphereTraceByChannel _returnvalue_3 (- _returnvalue_3 "0.000000,0.000000,50.000000") 2e+01 "TraceTypeQuery1" false 0 (Variables|WallRunningDebug|GetInitialGroundTraceDebug)))
        (if (not _returnvalue_5)
          (if (Variables|WallRunningCustomisable|GetUseGripTimer?)
            (if (and (!= (Components|Timeline|GetPlaybackPosition (Variables|Default|GetGripTimer)) 1.0) (not (Variables|WallRunningCustomisable|GetLockGripTimer)))
              (CallFunction|StartGripTimer)
              (CallFunction|StartWallRun :!label _label))
            (else
              (goto _label))))))))

(event OnComponentBeginOverlap(CapsuleComponent)
  (params (OverlappedComponent :type Primitive%20Component%20Object%20Reference) (OtherActor :type Actor%20Object%20Reference) (OtherComp :type Primitive%20Component%20Object%20Reference) (OtherBodyIndex :type Integer) (bFromSweep :type Boolean) (SweepResult :type Hit%20Result%20Structure%20%28by%20ref%29))
  (bind _tutorial (Variables|Default|GetTutorial))
  ;[0.15 0 0.1189 0.5] Finish Line Logic
  (|IsTutorial_2_3
    (:then
      (if (not (Actor|ActorHasTag OtherActor "Fin"))
        (if (Actor|ActorHasTag OtherActor "Destroy")
          (Class|FMODBlueprintStatics|PlayEventatLocation "/Game/FMOD/Events/Item.Item" (Math|Conversions|ToTransform(Vector) (Transformation|GetActorLocation)))
          (Widget|SetVisibility _tutorial "Collapsed")
          (else
            (Default|DefineText (Variables|Default|GetTutorial) (Utilities|String|ToString(Name) (Utilities|Array|Get(acopy) (Variables|/Script/Engine.Actor|GetTags OtherActor))))
            (Widget|SetVisibility _tutorial "Visible")))))
    (:else
      (if (Utilities|DoesObjectImplementInterface OtherActor "/Game/Core/Map2/FinishLine/TimerInterface_BP.TimerInterface_BP_C")
        (Default|StopStopWatch (Variables|Default|GetTimerUI))))))

(event Custom|WallRunRotation
  ;[0 0.008023 0.15 0.502] Wallrun
  ;;[0 0.01161 0.15 0.502] Align Player to wall while Wall Running
  (Transformation|SetActorRotation (Math|Interpolation|RInterpTo (Transformation|GetActorRotation) (Math|Rotator|MakeRotfromX (Variables|WallRunning|GetWallRunNormal)) (Utilities|Time|GetWorldDeltaSeconds) 15.0)))

(event Custom|SetWallrunOptions
  (params (Gravity%20Scale :type Float%20%28single-precision%29) (PlaneConstraintEnabled :type Boolean) (PlaneNormal :type Vector) (Orient%20Rotation%20to%20Movement :type Boolean) (Radius :type Float%20%28single-precision%29) (WallRunning :type Boolean))
  (bind _charactermovement (Variables|Character|GetCharacterMovement))
  ;[0 0.008023 0.15 0.502] Wallrun
  ;;[0 0.008023 0.15 0.502] Sets Initial Values
  (Variables|/Script/Engine.CharacterMovementComponent|SetGravityScale _charactermovement Gravity%20Scale)
  (Class|MovementComponent|SetPlaneConstraintEnabled _charactermovement PlaneConstraintEnabled)
  (Class|MovementComponent|SetPlaneConstraintNormal _charactermovement PlaneNormal)
  (Variables|/Script/Engine.CharacterMovementComponent|SetbOrientRotationToMovement _charactermovement Orient%20Rotation%20to%20Movement)
  (Variables|Default|SetbIsWallRunning WallRunning)
  (Components|Capsule|SetCapsuleRadius (Variables|Default|GetCapsuleComponent) Radius true))

(event Custom|StartWallRun
  (bind _returnvalue (Transformation|GetActorForwardVector))
  (bind _returnvalue_2 (Transformation|GetVelocity))
  (bind _wallrunningminimumspeed (Variables|WallRunningCustomisable|GetWallRunningMinimumSpeed))
  (bind _returnvalue_3 (Math|Vector|DotProduct _returnvalue_2 _returnvalue))
  ;[0 0.008023 0.15 0.502] Wallrun
  ;;[0 0.008023 0.15 0.502] Start and end Wallrun. Set the variables and use timelines for grip strength and gravity
  (if (not (Variables|WallRunning|GetWallRunningCoolDown))
    (CallFunction|SetWallrunOptions 0.0 true "0.000000,0.000000,1.000000" false 45.0 true)
    (if (Utilities|Enum|Equal(Enum) (Variables|WallRunning|GetWallRunDirection) "NewEnumerator0")
      _
      (else
        _))
    (if (< (Class|TaraCharacter|GetCurrentSatchels) 1)
      (Variables|Default|SetCurrentSatchels 1.0)
      (Class|TaraCharacter|BroadcastCurrentStats))
    (if (or (< _returnvalue_3 (* _wallrunningminimumspeed -1.0)) (> _returnvalue_3 _wallrunningminimumspeed))
      (Utilities|FlowControl|Sequence
        (:then_0
          (if (Variables|WallRunningCustomisable|GetUseGripTimer?)
            (Utilities|FlowControl|Sequence
              (:then_0
                (Default|PlayFade (Variables|WallRunningCustomisable|GetGripTimerUi) "Forward"))
              (:then_1
                (Components|Timeline|SetPlayRate (Variables|Default|GetGripTimer) 1.0)
                (bind (_direction _newtrack_0) (Timeline|GripTimer Play)
                  (:Update
                    (Progress|SetPercent (Variables|/Game/Core/Wallrun/GripTimer.GripTimer_C|GetProgressBar_0 (Variables|WallRunningCustomisable|GetGripTimerUi)) (Math|Float|Lerp 1.0 0.0 _newtrack_0)))
                  (:Finished
                    (CallFunction|ResetWallrun)
                    (switch Utilities|FlowControl|Switch|SwitchonETimelineDirection _direction
                      (:Forward
                        (Variables|WallRunningCustomisable|SetLockGripTimer true)
                        (Default|OnTimerEnd (Variables|WallRunningCustomisable|GetGripTimerUi)))
                      (:Backward
                        (Variables|WallRunningCustomisable|SetLockGripTimer false)))))))))
        (:then_1
          (Utilities|FlowControl|RetriggerableDelay 0.2)
          (Variables|WallRunning|SetTraceForward? true))
        (:then_2
          (bind _value (Timeline|Arc PlayFromStart)
            (:Update
              (Transformation|AddActorWorldOffset (Math|Vector|MakeVector 0.0 0.0 _value))))))
      (else
        (CallFunction|ResetWallrun)))))

(event Custom|StartGripTimer
  ;[0 0.008023 0.15 0.502] Wallrun
  ;;[0 0.008023 0.15 0.502] Start and end Wallrun. Set the variables and use timelines for grip strength and gravity
  (Components|Timeline|SetPlayRate (Variables|Default|GetGripTimer) 1.0)
  (bind (_direction _newtrack_0) (Timeline|GripTimer Play)
    (:Update
      (Progress|SetPercent (Variables|/Game/Core/Wallrun/GripTimer.GripTimer_C|GetProgressBar_0 (Variables|WallRunningCustomisable|GetGripTimerUi)) (Math|Float|Lerp 1.0 0.0 _newtrack_0)))
    (:Finished
      (CallFunction|ResetWallrun)
      (switch Utilities|FlowControl|Switch|SwitchonETimelineDirection _direction
        (:Forward
          (Variables|WallRunningCustomisable|SetLockGripTimer true)
          (Default|OnTimerEnd (Variables|WallRunningCustomisable|GetGripTimerUi)))
        (:Backward
          (Variables|WallRunningCustomisable|SetLockGripTimer false))))))

(event Custom|ReverseGripTimer
  ;[0 0.008023 0.15 0.502] Wallrun
  ;;[0 0.008023 0.15 0.502] Start and end Wallrun. Set the variables and use timelines for grip strength and gravity
  (Components|Timeline|SetPlayRate (Variables|Default|GetGripTimer) 0.5)
  (bind (_direction _newtrack_0) (Timeline|GripTimer Reverse)
    (:Update
      (Progress|SetPercent (Variables|/Game/Core/Wallrun/GripTimer.GripTimer_C|GetProgressBar_0 (Variables|WallRunningCustomisable|GetGripTimerUi)) (Math|Float|Lerp 1.0 0.0 _newtrack_0)))
    (:Finished
      (CallFunction|ResetWallrun)
      (switch Utilities|FlowControl|Switch|SwitchonETimelineDirection _direction
        (:Forward
          (Variables|WallRunningCustomisable|SetLockGripTimer true)
          (Default|OnTimerEnd (Variables|WallRunningCustomisable|GetGripTimerUi)))
        (:Backward
          (Variables|WallRunningCustomisable|SetLockGripTimer false))))))

(event Custom|ResetWallrun
  ;[0 0.008023 0.15 0.502] Wallrun
  ;;[0 0.008023 0.15 0.502] Start and end Wallrun. Set the variables and use timelines for grip strength and gravity
  (CallFunction|SetWallrunOptions 2.25 false "0, 0, 0" false 35.0 false)
  (Transformation|SetRelativeRotation (Variables|Character|GetMesh) "0.000000,-90.000000,0.000000" false false)
  (Utilities|FlowControl|Sequence
    (:then_0
      (Variables|WallRunning|SetTraceForward? false)
      (bind _value (Timeline|Arc Stop)
        (:Update
          (Transformation|AddActorWorldOffset (Math|Vector|MakeVector 0.0 0.0 _value)))))
    (:then_1
      (if (Variables|WallRunningCustomisable|GetUseGripTimer?)
        (CallFunction|ReverseGripTimer)))))

(event Custom|NewKey
  (params (Collectible :type String))
  ;[0.9646 0.9792 0 0.5] Saving
  (Variables|Default|SetCollectible Collectible))

(event Input|EnhancedActionEvents|EnhancedInputActionPauseGame
  (params (ActionValue :type Boolean) (ElapsedSeconds :type Float%20%28double-precision%29) (TriggeredSeconds :type Float%20%28double-precision%29) (InputAction :type Input%20Action%20Object%20Reference :default "/Game/Core/Input/PauseGame.PauseGame"))
  ;[0.5573 0.4318 0.1742 0.5] PauseLogic
  (|IsTutorial_2_2
    (:else
      (Default|StopStopWatch (Variables|Default|GetTimerUI)))))

(event Input|EnhancedActionEvents|EnhancedInputActionSatchel
  (params (ActionValue :type Boolean) (ElapsedSeconds :type Float%20%28double-precision%29) (TriggeredSeconds :type Float%20%28double-precision%29) (InputAction :type Input%20Action%20Object%20Reference :default "/Game/Core/Input/Satchel.Satchel"))
  (bind _returnvalue (Class|TaraCharacter|GetCurrentSatchels))
  ;[1 0.07252 0 0.5] Satchel Logic
  (if (Variables|Default|GetCanThrowSatchel)
    (Utilities|IsValid (Variables|Default|GetSatchel)
      (:Is%20Valid
        (Variables|Default|SetActiveSatchels (- (Variables|Default|GetActiveSatchels) 1))
        (Variables|Default|SetbIsSatchelActive false)
        (Class|TaraCharacter|BroadcastCurrentStats)
        (Default|Detonate (Variables|Default|GetSatchel)))
      (:Is%20Not%20Valid
        (if (>= _returnvalue 1)
          (Variables|Default|SetCurrentSatchels (Math|Conversions|ToFloat(Integer) (- _returnvalue 1)))
          (Variables|Default|SetActiveSatchels (+ (Variables|Default|GetActiveSatchels) 1))
          (bind _returnvalue_2 (Game|SpawnActorfromClass "/Game/Core/Satchel/Satchel_BP.Satchel_BP_C" (Math|Transform|MakeTransform (+ (Transformation|GetWorldLocation (Variables|Default|GetCapsuleComponent)) (* (Math|Vector|GetForwardVector (Variables|Default|GetCameraComp)) 50)) (Transformation|GetActorRotation) "0.500000,0.500000,0.500000") "Undefined" "MultiplyWithRoot" 0 0))
          (bind _output_get (Variables|Default|SetSatchel _returnvalue_2))
          (Default|ThrowSatchel _output_get (Math|Vector|GetForwardVector (Variables|Default|GetCameraComp)))
          (Variables|Default|SetbIsSatchelActive true)
          (Class|TaraCharacter|BroadcastCurrentStats))))))

(event Input|EnhancedActionEvents|EnhancedInputActionJump
  (params (ActionValue :type Boolean) (ElapsedSeconds :type Float%20%28double-precision%29) (TriggeredSeconds :type Float%20%28double-precision%29) (InputAction :type Input%20Action%20Object%20Reference :default "/Game/Core/Input/Jump.Jump"))
  (bind _returnvalue (Transformation|GetVelocity))
  ;[0 0.008023 0.15 0.502] Wallrun
  ;;[0 0.01161 0.15 0.502] WallJump
  (:Started
    (if (Variables|Default|GetbIsWallRunning)
      (Character|LaunchCharacter (+ (* (Variables|WallRunning|GetWallSurfaceNormal) 1e+03) (Math|Vector|MakeVector (.x _returnvalue) (.y _returnvalue) 1e+03)) true true)
      (CallFunction|ResetWallrun)
      (Variables|/Script/Engine.CharacterMovementComponent|SetGravityScale (Variables|Character|GetCharacterMovement) (Variables|Default|GetNormalGravity))
      (if (Variables|WallRunningCustomisable|GetUseGripTimer?)
        (CallFunction|ReverseGripTimer)))))

(event EventTick
  (params (DeltaSeconds :type Float%20%28single-precision%29))
  ;[0.06629 0.15 0 0.5] TICK
  (Class|TaraCharacter|BroadcastCurrentStats)
  (if (|IsOnGroundAndWithoutSatchelsActive)
    (Variables|Default|SetCurrentSatchels 2.0))
  (if (Variables|Default|GetbIsWallRunning)
    (CallFunction|WallRunRotation)
    (CallFunction|WallRunTick)))

(event EventBeginPlay
  ;[0 0.008023 0.15 0.502] Wallrun
  ;;[0 0.008023 0.15 0.502] If using grip use widget
  (bind _astara_controller (Utilities|Casting|CastToTaraController (Pawn|GetController)))
  (Variables|/Script/BotBlastFinal.TaraController|SetbCanJump _astara_controller false)
  (Variables|/Script/BotBlastFinal.TaraController|SetMovementLock _astara_controller 0)
  (if (Variables|WallRunningCustomisable|GetUseGripTimer?)
    (bind _returnvalue (UserInterface|CreateWidget "/Game/Core/Wallrun/GripTimer.GripTimer_C"))
    (bind _output_get (Variables|WallRunningCustomisable|SetGripTimerUi _returnvalue))
    (UserInterface|Viewport|AddtoViewport _output_get 0))
  (|IsTutorial
    (:then
      _)
    (:else
      (bind _returnvalue_2 (UserInterface|CreateWidget "/Game/Core/BB_UI/Timer/StopWatch.StopWatch_C"))
      (bind _output_get_2 (Variables|Default|SetTimerUI _returnvalue_2))
      (UserInterface|Viewport|AddtoViewport _output_get_2 0)
      (Utilities|FlowControl|Delay 1.0)))
  (Variables|/Script/BotBlastFinal.TaraController|SetMovementLock _astara_controller 1)
  (Variables|/Script/BotBlastFinal.TaraController|SetbCanJump _astara_controller true)
  (Variables|Default|SetCanThrowSatchel true)
  (|IsTutorial_2_2_2
    (:then
      (bind _returnvalue_3 (UserInterface|CreateWidget "/Game/Core/BB_UI/Menu/TutorialDialogue.TutorialDialogue_C"))
      (bind _output_get_3 (Variables|Default|SetTutorial _returnvalue_3))
      (UserInterface|Viewport|AddtoViewport _output_get_3 -1))))

(event EventOnLanded
  (params (Hit :type Hit%20Result%20Structure%20%28by%20ref%29))
  ;[1 0.07252 0 0.5] Satchel Logic
  (Variables|Default|SetCurrentSatchels 2.0)
  (Class|TaraCharacter|BroadcastCurrentStats)
  (bind _astara_controller (Utilities|Casting|CastToTaraController (Pawn|GetController)))
  (Variables|/Script/BotBlastFinal.TaraController|SetbCanJump _astara_controller true))

(event EventRestartTimer
  ;[0.5573 0.4318 0.1742 0.5] PauseLogic
  (|IsTutorial_2
    (:else
      (Default|RestartStopWatch (Variables|Default|GetTimerUI)))))

(event EventSaveTime
  (params (Time :type Float%20%28double-precision%29))
  ;[0.9646 0.9792 0 0.5] Saving
  (Class|BotBlastBluePrintLibrary|SaveCollectibleKeys (Variables|Default|GetCollectible))
  (Development|PrintString "Saved" true true "(R=0.000000,G=0.660000,B=1.000000,A=1.000000)" 2e+01)
  (bind _returnvalue (Game|GetCurrentLevelName true))
  (Development|PrintString _returnvalue)
  (Class|BotBlastBluePrintLibrary|SaveLeaderboard _returnvalue "Jommy" (Variables|/Game/Core/BB_UI/Timer/StopWatch.StopWatch_C|GetTime (Variables|Default|GetTimerUI))))

(fn ConstructionScript)

(fn ContinueWallrun?
  (bind _returnvalue (Input|EnhancedActionValues|GetMove))
  ;[0.15 0.15 0.15 0.5] Find if should continue wallrun depending on inputs
  (return (or (Math|Float|NearlyEqual(Float) (.x _returnvalue) (Utilities|Select :Index (Variables|WallRunning|GetWallRunDirection) :NewEnumerator0 1.0 :NewEnumerator1 -1.0) 1e-06) (> (.y _returnvalue) 0.0))))

(fn GetInputDirection
  (bind _returnvalue (Pawn|GetControlRotation :!class /Script/Engine.Pawn))
  (bind _returnvalue_2 (Input|EnhancedActionValues|GetMove))
  (bind _returnvalue_3 (Input|EnhancedActionValues|GetMove))
  (bind _returnvalue_4 (Math|Vector|MakeVector (.x _returnvalue_3) (.y _returnvalue_3) 0.0))
  (bind _yaw (Math|Vector|GetYawPitchfromVector _returnvalue_4))
  (bind _returnvalue_5 (Math|Rotator|MakeRotator 0.0 0.0 _yaw))
  (bind _returnvalue_6 (Math|Rotator|Delta(Rotator) _returnvalue _returnvalue_5))
  (bind _returnvalue_7 (+ (.yaw _returnvalue_6) 9e+01))
  (return (Math|Rotator|MakeRotator 0.0 0.0 (Math|Float|SelectFloat _returnvalue_7 (.yaw (Math|Conversions|RotationFromXVector (Transformation|GetActorForwardVector))) (!= (+ (.x _returnvalue_2) (.y _returnvalue_2)) 0.0))) (Math|Rotator|MakeRotator 0.0 0.0 _returnvalue_7)))

(fn WallRunTick
  (bind _returnvalue (Transformation|GetActorLocation))
  (bind _returnvalue_2 (Transformation|GetActorRightVector))
  (bind _returnvalue_3 (Transformation|GetActorLocation))
  (bind _returnvalue_4 (Transformation|GetActorForwardVector))
  (bind _mesh (Variables|Character|GetMesh))
  (bind _wallrundirection (Variables|WallRunning|GetWallRunDirection))
  (bind _returnvalue_5 (Transformation|GetWorldLocation _mesh))
  (bind _returnvalue_6 (* _returnvalue_4 5e+01))
  (bind _returnvalue_7 (Utilities|Select :Index _wallrundirection :NewEnumerator0 1.0 :NewEnumerator1 -1.0))
  (bind _returnvalue_8 (* _returnvalue_2 _returnvalue_7 5.0))
  (bind _returnvalue_9 (+ _returnvalue_3 _returnvalue_6))
  (bind _returnvalue_10 (+ _returnvalue_5 _returnvalue_8))
  ;[0 0.02302 0.15 0.5] Do initial traces, and if can continue then trace for the wall being run on.
  (if (CallFunction|ContinueWallrun?)
    (bind _returnvalue_11 (Collision|SphereTraceByChannel _returnvalue_5 (+ _returnvalue_5 (* _returnvalue_2 _returnvalue_7 6e+01)) 5.0 "TraceTypeQuery1" false 0 (Variables|WallRunningDebug|GetFootCheckDebug)))
    (bind _returnvalue_12 (Collision|SphereTraceByChannel _returnvalue_10 _returnvalue_10 1e+01 "TraceTypeQuery1" false 0 (Variables|WallRunningDebug|GetGroundCheckDebug)))
    (bind _returnvalue_13 (Collision|CapsuleTraceByChannel _returnvalue_9 _returnvalue_9 (Math|Float|SelectFloat 1e+01 0.0 (Variables|WallRunning|GetTraceForward?)) 5e+01 "TraceTypeQuery1" false 0 (Variables|WallRunningDebug|GetForwardCheckDebug)))
    (if (Math|Boolean|ANDBoolean _returnvalue_11 (not _returnvalue_12) (not _returnvalue_13))
      (Utilities|FlowControl|Sequence
        (:then_0
          (bind (_outhit _returnvalue_14) (Collision|LineTraceByChannel _returnvalue (+ _returnvalue (* (Math|Vector|CrossProduct (Variables|WallRunning|GetWallRunNormal) (Utilities|Select :Index (Variables|WallRunning|GetWallRunDirection) :NewEnumerator0 "0.000000,0.000000,-1.000000" :NewEnumerator1 "0.000000,0.000000,1.000000")) 2e+02)) "TraceTypeQuery1" false 0 "ForOneFrame"))
          (if _returnvalue_14
            (Variables|WallRunning|SetWallSurfaceNormal (.ImpactNormal (Collision|BreakHitResult _outhit)))
            (Variables|WallRunning|SetWallRunNormal (Math|Vector|CrossProduct (.ImpactNormal (Collision|BreakHitResult _outhit)) (Utilities|Select :Index (Variables|WallRunning|GetWallRunDirection) :NewEnumerator0 "0.000000,0.000000,-1.000000" :NewEnumerator1 "0.000000,0.000000,1.000000"))))))
      (else
        (CallFunction|ResetWallrun)))
    (else
      (CallFunction|ResetWallrun))))