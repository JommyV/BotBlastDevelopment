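; Satchel_BP is a thrown satchel charge projectile that detonates on a timer.
; ThrowSatchel launches it along the given direction at the projectile's initial speed, adding half the instigator's velocity so throws inherit the thrower's momentum.
; After a three-second delay, Detonate fires a radial force impulse and destroys the actor.
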(event Custom|Detonate
  (Class|RadialForceComponent|FireImpulse (Variables|Default|GetRadialForce))
  (Actor|DestroyActor))

(event Custom|ThrowSatchel
  (params (Direction :type Vector))
  (Variables|/Script/Engine.MovementComponent|SetVelocity (Variables|Default|GetProjectileMovement) (+ (* Direction (Variables|/Script/Engine.ProjectileMovementComponent|GetInitialSpeed (Variables|Default|GetProjectileMovement))) (* (Transformation|GetVelocity (Game|GetInstigator)) 0.5)))
  (Utilities|FlowControl|Delay 3.0)
  (CallFunction|Detonate))

(fn ConstructionScript)