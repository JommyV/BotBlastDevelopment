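; BotBlastKey_BP is a key actor that adds its KeyString to the player's key wallet when any actor overlaps it.
; On BeginPlay it caches the player's TaraCharacter and binds to its OnKeyWalletAction dispatcher, and overlap calls AddKey on that reference.
; The wallet callback compares key strings and prints the string on both success and failure, with no destroy or hide logic.
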(event Custom|OnKeyWalletAction_Event_0
  (params (KeyString :type String) (KeyAction :type EPlayerKeyAction%20Enum :default "AddKey") (IsSuccess :type Boolean))
  (if (Utilities|Enum|Equal(Enum) KeyString (Variables|Default|GetKeyString))
    (if IsSuccess
      (Development|PrintString KeyString true true "(R=0.000000,G=1.000000,B=0.081256,A=1.000000)")
      (else
        (Development|PrintString KeyString true true "(R=0.604167,G=0.016324,B=0.000000,A=1.000000)")))))

(event EventBeginPlay
  (bind _astara_character (Utilities|Casting|CastToTaraCharacter (Game|GetPlayerCharacter 0)))
  (bind _output_get (Variables|Default|SetTaraCharacterReference _astara_character))
  (EventDispatchers|AssignOnKeyWalletAction _output_get (delegate Custom|OnKeyWalletAction_Event_0)))

(event EventTick
  (params (DeltaSeconds :type Float%20%28single-precision%29)))

(event Collision|EventActorBeginOverlap
  (params (OtherActor :type Actor%20Object%20Reference))
  (Class|TaraCharacter|AddKey (Variables|Default|GetTaraCharacterReference) (Variables|Default|GetKeyString)))

(fn ConstructionScript)